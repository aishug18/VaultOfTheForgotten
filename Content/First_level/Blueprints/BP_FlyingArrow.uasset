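; BP_FlyingArrow is an arrow trap that animates back and forth and hurts the player on contact.
; On BeginPlay it saves the arrow's relative location, then a timeline lerps its X toward EndX while holding Y and Z.
; When the arrow begins overlapping a BP_ThirdPersonCharacter, it calls that character's EnvironmentTakeDamage with a fixed amount.
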(event OnComponentBeginOverlap(OS_Arrow)
  (params (OverlappedComponent :type Primitive%20Component%20Object%20Reference) (OtherActor :type Actor%20Object%20Reference) (OtherComp :type Primitive%20Component%20Object%20Reference) (OtherBodyIndex :type Integer) (bFromSweep :type Boolean) (SweepResult :type Hit%20Result%20Structure%20%28by%20ref%29))
  ;[0.15 0.15 0.15 0.5] Cause damage when in contact
  (bind _asbp_third_person_character (Utilities|Casting|CastToBP_ThirdPersonCharacter OtherActor))
  (Default|EnvironmentTakeDamage _asbp_third_person_character 2e+01))

(event EventBeginPlay
  ;[0.15 0.15 0.15 0.5] Save current location
  (Variables|Default|SetCurrent%20Location (Variables|/Script/Engine.SceneComponent|GetRelativeLocation (Variables|Default|GetOS_Arrow)))
  ;[0.15 0.15 0.15 0.5] Move arrow back and forth using timeline to animate
  (bind _launch (Timeline|Timeline Play)
    (:Update
      (Transformation|SetRelativeLocation (Variables|Default|GetOS_Arrow) (Math|Vector|MakeVector (Math|Float|Lerp (.x (Variables|Default|GetCurrent%20Location)) (Variables|Default|GetEndX) _launch) (.y (Variables|Default|GetCurrent%20Location)) (.z (Variables|Default|GetCurrent%20Location))) false false))))

(fn ConstructionScript)