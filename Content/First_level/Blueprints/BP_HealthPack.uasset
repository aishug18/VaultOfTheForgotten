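; BP_HealthPack is a pickup actor that heals the third-person player character when touched.
; On overlap it casts to BP_ThirdPersonCharacter and, only if health is below full, calls the damage system component's Heal and writes back the Health value.
; It then destroys itself and plays a heal sound and Niagara effect at its location, so a full-health player leaves the pack in place.
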(event Collision|EventActorBeginOverlap
  (params (OtherActor :type Actor%20Object%20Reference))
  (bind _returnvalue (Transformation|GetActorLocation))
  ;[0.15 0.15 0.15 0.5] Add 30 to Player Health and destroy the Health Pack
  (bind _asbp_third_person_character (Utilities|Casting|CastToBP_ThirdPersonCharacter OtherActor))
  (if (< (Variables|/Game/First_level/Combat/DamageSystem/BPC_DamageSystem.BPC_DamageSystem_C|GetHealth (Variables|/Game/ThirdPerson/Blueprints/BP_ThirdPersonCharacter.BP_ThirdPersonCharacter_C|GetBPC_DamageSystem _asbp_third_person_character)) 1e+02)
    (bind _newhealth (Default|Heal (Variables|/Game/ThirdPerson/Blueprints/BP_ThirdPersonCharacter.BP_ThirdPersonCharacter_C|GetBPC_DamageSystem _asbp_third_person_character) 3e+01))
    (Variables|/Game/First_level/Combat/DamageSystem/BPC_DamageSystem.BPC_DamageSystem_C|SetHealth (Variables|/Game/ThirdPerson/Blueprints/BP_ThirdPersonCharacter.BP_ThirdPersonCharacter_C|GetBPC_DamageSystem _asbp_third_person_character) _newhealth)
    (Actor|DestroyActor)
    (Audio|PlaySoundatLocation "/Game/First_level/Audio/heal_Cue.heal_Cue" _returnvalue "0, 0, 0" 1.0 1.0 0.0 0 0 0 0)
    (Niagara|SpawnSystematLocation "/Game/First_level/Blueprints/NS_Heal.NS_Heal" _returnvalue)))

(fn ConstructionScript)