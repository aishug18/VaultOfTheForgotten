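; Base enemy character, apparently a zombie, with melee attack, patrol route, speed tiers and an overhead health bar widget.
; Health, healing and damage delegate to BPCDamageSystem, whose death event enables mesh physics and later destroys the actor.
; Attack plays a punch montage and timed Niagara effect, signals attack end, then sphere-traces forward to damage pawns through a damage message.
; The damage response handler is empty.
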(event Custom|Attack
  (bind _returnvalue (Transformation|GetActorLocation))
  (bind _returnvalue_2 (Transformation|GetActorForwardVector))
  (bind _returnvalue_3 (* _returnvalue_2 1e+02))
  (bind _returnvalue_4 (+ _returnvalue _returnvalue_3))
  ;[0.15 0.15 0.15 0.5] Attack player, play animation
  (if (not (Variables|/Game/First_level/Combat/DamageSystem/BPC_DamageSystem.BPC_DamageSystem_C|GetIsDead (Variables|Default|GetBPC_DamageSystem)))
    (Utilities|Casting|CastToBP_EnemyAnim (Components|SkeletalMesh|GetAnimInstance (Variables|Character|GetMesh)))
    (Animation|PlayAnimMontage "/Game/First_level/Assets/Enemies/Mummy/Animations/ZombiePunchMontage.ZombiePunchMontage" 1.0 "None")
    (Utilities|FlowControl|Delay 0.6)
    (bind _returnvalue_5 (Niagara|SpawnSystematLocation "/Game/First_level/Combat/NS_EnemyAttack.NS_EnemyAttack" _returnvalue_4))
    (Utilities|FlowControl|Delay 0.4)
    (Default|CallOnAttackEnd)
    (Components|DestroyComponent _returnvalue_5)
    (bind (_outhit _returnvalue_6) (Collision|SphereTraceForObjects _returnvalue _returnvalue_4 7e+01 (Utilities|Array|MakeArray "ObjectTypeQuery3") false 0 "None" true "(R=1.000000,G=0.110250,B=0.726213,A=1.000000)" "(R=0.000000,G=0.684448,B=1.000000,A=1.000000)" 1.0))
    (if _returnvalue_6
      (Class|BPIDamagable|TakeDamage(Message) (.HitActor (Collision|BreakHitResult _outhit)) (Utilities|Struct|MakeS_DamageInfo 1e+01 "NewEnumerator1" "NewEnumerator1")))))

(event Custom|Death
  (bind _mesh (Variables|Character|GetMesh))
  ;[0.15 0.15 0.15 0.5] Die and play death animation, then destroy actor
  (Physics|SetSimulatePhysics _mesh true)
  (Collision|SetCollisionEnabled _mesh "QueryAndPhysics")
  (Utilities|FlowControl|Delay 3.5)
  (Actor|DestroyActor))

(event Custom|DamageResponse
  (params (DamageResponse :type E_DamageResponse%20Enum :default "NewEnumerator0")))

(event EventBeginPlay
  ;[0.15 0.15 0.15 0.5] Add health bar widget to the top of enemy head
  (bind _returnvalue (UserInterface|CreateWidget "/Game/First_level/Combat/DamageSystem/WB_EnemyHealthBar.WB_EnemyHealthBar_C" 0 self))
  (UserInterface|SetWidget (Variables|Default|GetHealthWidget) _returnvalue))

(fn ConstructionScript
  (bind _bpc_damagesystem (Variables|Default|GetBPC_DamageSystem))
  (EventDispatchers|BindEventtoOnDeath _bpc_damagesystem (EventDispatchers|CreateEvent :!event Custom|Death))
  (EventDispatchers|BindEventtoOnDamageResponse _bpc_damagesystem (EventDispatchers|CreateEvent :!event Custom|DamageResponse)))

(fn GetCurrentHealth
  (return (Variables|/Game/First_level/Combat/DamageSystem/BPC_DamageSystem.BPC_DamageSystem_C|GetHealth (Variables|Default|GetBPC_DamageSystem))))

(fn GetMaxHealth
  (return (Variables|/Game/First_level/Combat/DamageSystem/BPC_DamageSystem.BPC_DamageSystem_C|GetMaxHealth (Variables|Default|GetBPC_DamageSystem))))

(fn GetPatrolRoute
  (return (Variables|AI|GetPatrolRoute)))

(fn Heal
  (params (Amount :type Float%20%28double-precision%29))
  (bind _newhealth (Default|Heal (Variables|Default|GetBPC_DamageSystem) Amount))
  (return _newhealth))

(fn SetMovementSpeed
  (params (Speed :type E_MovementSpeed%20Enum :default "NewEnumerator0"))
  (bind _output_get (Variables|/Script/Engine.CharacterMovementComponent|SetMaxWalkSpeed (Variables|Character|GetCharacterMovement) (Utilities|Select :Index Speed :NewEnumerator0 0.0 :NewEnumerator1 1e+02 :NewEnumerator2 2e+02 :NewEnumerator3 3e+02)))
  (return _output_get))

(fn TakeDamage
  (params (DamageInfo :type S%20Damage%20Info%20Structure))
  (bind _wasdamaged (Default|TakeDamage (Variables|Default|GetBPC_DamageSystem) DamageInfo))
  (return _wasdamaged))