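; BP_PatrolRoute is a spline-based patrol path actor in the first level's combat AI.
; It tracks a current point index and returns that spline point's world position through GetSplinePointAsWorldPosition.
; IncrementPatrolRoute steps the index by a direction value, which flips at the last and first points so the route runs back and forth instead of looping.
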(event Custom|IncrementPatrolRoute
  ;[0.15 0.15 0.15 0.5] Increment position to move
  (bind _output_get (Variables|Default|SetPatrolIndex (+ (Variables|Default|GetPatrolIndex) (Variables|Default|GetDirection))))
  ;[0.15 0.15 0.15 0.5] Reached end of route, so go backwards
  (if (== _output_get (- (Spline|GetNumberOfSplinePoints (Variables|Default|GetPatrolRoute)) 1))
    (Variables|Default|SetDirection -1)
    (else
      ;[0.15 0.15 0.15 0.5] Reached beginning of route, so go forward
      (if (== (Variables|Default|GetPatrolIndex) 0)
        (Variables|Default|SetDirection 1)))))

(fn ConstructionScript)

(fn GetSplinePointasWorldPosition
  (return (Spline|GetLocationatSplinePoint (Variables|Default|GetPatrolRoute) (Variables|Default|GetPatrolIndex) "World")))