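; BP_OS_Enemy is an enemy that chases the player on sight and damages them when it arrives.
; PawnSensing sets a seeing flag, which is never cleared here, and starts an AI MoveTo toward player zero.
; On success it casts the pawn to the third-person character and calls DamageTaken.
; Incoming damage overwrites Health rather than subtracting from it, then prints it; at zero or below it only prints a placeholder message.
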(event OnSeePawn(PawnSensing)
  (params (Pawn :type Pawn%20Object%20Reference))
  (Variables|Default|SetinSeeingPlayer true)
  (CallFunction|FollowPlayer))

(event Custom|Follow%20Player
  (if (Variables|Default|GetinSeeingPlayer)
    (AI|AIMoveTo self "0, 0, 0" (Game|GetPlayerCharacter 0) 5.0 false
      (:OnSuccess
        (bind _asbp_os_third_person_character_1 (Utilities|Casting|CastToBP_OS_ThirdPersonCharacter1 (stale OnSeePawn(PawnSensing) Pawn)))
        (Default|DamageTaken _asbp_os_third_person_character_1 (Variables|Default|Getdamage))))))

(event EventBeginPlay)

(event Collision|EventActorBeginOverlap
  (params (OtherActor :type Actor%20Object%20Reference)))

(event Game|Damage|EventAnyDamage
  (params (Damage :type Float%20%28single-precision%29) (DamageType :type Damage%20Type%20Object%20Reference) (InstigatedBy :type Controller%20Object%20Reference) (DamageCauser :type Actor%20Object%20Reference))
  (if (> (Variables|Default|Gethealth) 0.0)
    (bind _output_get (Variables|Default|Sethealth (- Damage 0.0)))
    (Development|PrintText (Utilities|Text|ToText(Float) _output_get "HalfToEven"))
    (else
      (Development|PrintText "Hello"))))

(fn ConstructionScript)